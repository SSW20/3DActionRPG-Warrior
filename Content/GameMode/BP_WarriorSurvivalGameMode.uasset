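; Survival game mode Blueprint that shows wave announcement UI as the game mode state changes.
; On BeginPlay it binds to OnGameModeStateChanged, routing waiting, spawning and completion states to functions that create viewport widgets.
; Waiting and completion widgets run a countdown from the wave wait threshold, with completion also showing the wave number.
; The start banner's branch is hardcoded true, always showing "Last Wave", and all-waves-complete only prints placeholder text.
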(event `self.ReceiveBeginPlay`
  (add `self.OnGameModeStateChanged` (delegate `OnGameModeStateChanged_이벤트`)))

(event `OnGameModeStateChanged_이벤트` :!signature `self.OnGameModeStateChanged`
  (params (GameModeState :type "ESurvivalGameModeState Enum" :default "WaitSpawnNewWave"))
  (switch `ESurvivalGameModeState` GameModeState
    (:`WaitSpawnNewWave`
      (`self.WaitNewWave`))
    (:`SpawningNewWave`
      (`self.StartNewWave`))
    (:`WaveComplete`
      (`self.WaveComplete`))
    (:`AllWavesComplete`
      (`KismetSystemLibrary.PrintString` "Hello"))))

(fn `StartNewWave`
  (locals (WaveStartWidget :type "/Game/GameMode/Wiget/WBP_NewWaveStart Object Reference"))
  (bind _returnvalue (`|CreateWidget` "/Game/GameMode/Wiget/WBP_NewWaveStart.WBP_NewWaveStart_C"))
  (set `local.WaveStartWidget` _returnvalue)
  (`UserWidget.AddToViewport` _returnvalue 0)
  (if true
    (set `TextBlock.Text` (`|FormatText` "Last Wave") (`/Game/GameMode/Wiget/WBP_NewWaveStart.WBP_WarriorTextBlock` (`local.WaveStartWidget`)))
    (`TextBlock.SetText` (`/Game/GameMode/Wiget/WBP_NewWaveStart.WBP_WarriorTextBlock_WaveCount` (`local.WaveStartWidget`)) "")
    (else
      (`TextBlock.SetText` (`/Game/GameMode/Wiget/WBP_NewWaveStart.WBP_WarriorTextBlock_WaveCount` (`local.WaveStartWidget`)) (`KismetTextLibrary.Conv_IntToText` (`self.CurrentWaveCount`))))))

(fn `UserConstructionScript`)

(fn `WaitNewWave`
  (bind _returnvalue (`|CreateWidget` "/Game/GameMode/Wiget/WBP_WaitNewWave.WBP_WaitNewWave_C"))
  (`UserWidget.AddToViewport` _returnvalue 0)
  (`/Game/GameMode/Wiget/WBP_WaitNewWave.CountDownEvent` _returnvalue (`self.WaitTimeNewWaveThreshold`)))

(fn `WaveComplete`
  (bind _returnvalue (`|CreateWidget` "/Game/GameMode/Wiget/WBP_WaitNewWave.WBP_WaitNewWave_C"))
  (`UserWidget.AddToViewport` _returnvalue 0)
  (`TextBlock.SetText` (`/Game/GameMode/Wiget/WBP_WaitNewWave.WBP_WarriorTextBlock` _returnvalue) (`|FormatText` "Wave {CurrentWaveCount} Complete!!" (`self.CurrentWaveCount`)))
  (`/Game/GameMode/Wiget/WBP_WaitNewWave.CountDownEvent` _returnvalue (`self.WaitTimeNewWaveThreshold`)))