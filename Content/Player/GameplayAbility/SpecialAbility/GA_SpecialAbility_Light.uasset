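; Gameplay ability for the hero's light axe special attack, combining a melee hit with a burning slash projectile.
; It plays the montage, commits and notifies the UI of the cooldown, and ends when the montage finishes or is interrupted.
; Montage-driven gameplay events spawn BP_BurningSlash from the weapon's slash socket, carrying a damage spec.
; Melee hit events apply damage, send a hit react, fire a gameplay cue and grant the owner rage.
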(event `self.K2_ActivateAbility`
  (bind _returnvalue (`self.GetCooldownTimeRemaining`))
  (`AbilityTask_PlayMontageAndWait.CreatePlayMontageAndWaitProxy` "None" "/Game/Player/AnimBP/AM_Hero_Axe_Ability_Light.AM_Hero_Axe_Ability_Light"
    (:`then`
      (`|ExecutionSequence`
        (:`then_0`
          (`AbilityTask_WaitGameplayEvent.WaitGameplayEvent` (struct :`TagName` "Shared.Event.SpawnProjectile") null
            (:`EventReceived`
              (`self.SpawnProjectile`))))
        (:`then_1`
          (bind (_asynctaskproxy _payload) (`AbilityTask_WaitGameplayEvent.WaitGameplayEvent` (struct :`TagName` "Shared.Event.MeleeHit") null)
            (:`EventReceived`
              (`self.HandleApplyDamage` _payload))))
        (:`then_2`
          (`self.K2_CommitAbility`)
          (`PlayerUIComponent.OnAbilityCoolDownChanged` (`WarriorPlayerCharacter.PlayerUIComponent` (`self.GetWarriorPlayerCharacterFromActorInfo`)) (struct :`TagName` "InputTag.SpecialWeaponAbility.Light") _returnvalue _returnvalue))))
    (:`OnCompleted`
      (`self.K2_EndAbility` :!label _label))
    (:`OnBlendOut`
      (goto _label))
    (:`OnInterrupted`
      (goto _label))
    (:`OnCancelled`
      (goto _label))))

(fn `HandleApplyDamage`
  (params (GameplayEvent :type "GameplayEventData Structure"))
  (locals (LocalTargetActor :type "Actor Object Reference") (GameplayCueTag :type "GameplayTag Structure" :default (struct :`TagName` "GameplayCue.Sound.Hit.Axe")))
  (bind _output_get (set `local.LocalTargetActor` (`.Target` (break `GameplayEventData` GameplayEvent))))
  (`self.BP_ApplyEffectToTarget` _output_get (`self.MakePlayerEffectSpecHandle` "/Game/Player/GameplayEffect/GE_Damage.GE_Damage_C" (`PlayerCombatComponent.GetEquippedWeaponBaseDamage` (`self.GetPlayerCombatComponentFromActorInfo`) (`KismetMathLibrary.Conv_IntToDouble` (`self.GetAbilityLevel`))) (struct :`TagName` "Player.SetByCaller.AttackType.Light") 4))
  (`AbilitySystemBlueprintLibrary.SendGameplayEventToActor` (`local.LocalTargetActor`) (struct :`TagName` "Shared.Event.HitReact") (`local.GameplayEvent`))
  (`self.K2_ExecuteGameplayCue` (`local.GameplayCueTag`))
  (`self.BP_ApplyGameplayEffectToOwner` "/Game/Player/GameplayEffect/GE_RageGain.GE_RageGain_C" (`self.GetAbilityLevel`)))

(fn `SpawnProjectile`
  (bind _returnvalue (`self.GetWarriorPlayerCharacterFromActorInfo`))
  (bind (_returnvalue_roll _returnvalue_pitch _returnvalue_yaw) (`KismetMathLibrary.BreakRotator` (`KismetMathLibrary.MakeRotFromX` (`Actor.GetActorForwardVector` (`self.GetWarriorPlayerCharacterFromActorInfo`)))))
  (bind _returnvalue_2 (`SceneComponent.GetSocketTransform` (`WarriorWeaponBase.WeaponMesh` (`PawnCombatComponent.GetCurrentEquippedWeapon` (`self.GetPlayerCombatComponentFromActorInfo`))) "SlashSocket" "RTS_World"))
  (`|SpawnActorFromClass` "/Game/Player/BP_BurningSlash.BP_BurningSlash_C" (`KismetMathLibrary.MakeTransform` (.location _returnvalue_2) (`KismetMathLibrary.MakeRotator` (.roll (.rotation _returnvalue_2)) 0.0 _returnvalue_yaw)) "AdjustIfPossibleButAlwaysSpawn" "MultiplyWithRoot" _returnvalue (`self.MakePlayerEffectSpecHandle` "/Game/Player/GameplayEffect/GE_Damage.GE_Damage_C" (`PlayerCombatComponent.GetEquippedWeaponBaseDamage` (`self.GetPlayerCombatComponentFromActorInfo`) (`KismetMathLibrary.Conv_IntToDouble` (`self.GetAbilityLevel`))) (struct :`TagName` "Player.SetByCaller.AttackType.Light") 1) _returnvalue))