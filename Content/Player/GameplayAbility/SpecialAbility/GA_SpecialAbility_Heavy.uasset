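; Gameplay ability for the player's heavy special weapon attack, an axe jump attack that deals area damage.
; It plays the jump montage and waits for the Shared.Event.AOE gameplay event, then calls HandleAOE, commits the ability and notifies the UI of the cooldown.
; HandleAOE sphere-traces ahead of the hero and applies a damage effect built from weapon base damage to the hits.
; The ability ends when the montage completes, blends out or is interrupted or cancelled.
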(event `self.K2_ActivateAbility`
  (bind _returnvalue (`self.GetCooldownTimeRemaining`))
  (`AbilityTask_PlayMontageAndWait.CreatePlayMontageAndWaitProxy` "None" "/Game/Player/Mongtages/AM_Hero_Axe_JumpAttack.AM_Hero_Axe_JumpAttack"
    (:`then`
      (`AbilityTask_WaitGameplayEvent.WaitGameplayEvent` (struct :`TagName` "Shared.Event.AOE") null
        (:`EventReceived`
          (`|ExecutionSequence`
            (:`then_0`
              (`self.HandleAOE`))
            (:`then_1`
              (`self.K2_CommitAbility`)
              (`PlayerUIComponent.OnAbilityCoolDownChanged` (`WarriorPlayerCharacter.PlayerUIComponent` (`self.GetWarriorPlayerCharacterFromActorInfo`)) (struct :`TagName` "InputTag.SpecialWeaponAbility.Heavy") _returnvalue _returnvalue))))))
    (:`OnCompleted`
      (`self.K2_EndAbility` :!label _label))
    (:`OnBlendOut`
      (goto _label))
    (:`OnInterrupted`
      (goto _label))
    (:`OnCancelled`
      (goto _label))))

(fn `HandleAOE`
  (bind _returnvalue (`self.GetWarriorPlayerCharacterFromActorInfo`))
  (bind _returnvalue_2 (+ (`Actor.K2_GetActorLocation` _returnvalue) (* (`Actor.GetActorForwardVector` _returnvalue) 200.0)))
  (bind _outhits (`KismetSystemLibrary.SphereTraceMultiForObjects` _returnvalue_2 _returnvalue_2 500.0 (`self.Object Types`)))
  (`self.ApplyEffectToTargetsByHitResults` _outhits (`self.MakePlayerEffectSpecHandle` "/Game/Player/GameplayEffect/GE_Damage.GE_Damage_C" (`PlayerCombatComponent.GetEquippedWeaponBaseDamage` (`self.GetPlayerCombatComponentFromActorInfo`) (`KismetMathLibrary.Conv_IntToDouble` (`self.GetAbilityLevel`))) (struct :`TagName` "Player.SetByCaller.AttackType.Heavy") 4)))