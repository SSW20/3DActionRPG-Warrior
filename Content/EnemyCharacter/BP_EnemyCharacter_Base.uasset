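; BP_EnemyCharacter_Base is the base enemy character Blueprint, implementing the death and dissolve sequence.
; OnEnemyDied pauses mesh animation, disables capsule collision, then async-loads and attaches the supplied Niagara effect, tinting its particles with the material's DissolveEdgeColor.
; Two timelines, rate-scaled by configurable durations, drive DissolveAmount on the body and equipped weapon materials, destroying each actor when its timeline finishes.
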(event `/Game/EnemyCharacter/BPI_EnemyDeathInterface.OnEnemyDied`
  (params (DeathNiagaraSystem :type "NiagaraSystem Soft Object Reference"))
  (bind _mesh (`self.Mesh`))
  (bind _weaponmesh (`WarriorWeaponBase.WeaponMesh` (`PawnCombatComponent.GetCurrentEquippedWeapon` (`self.EnemyCombatComponent`))))
  (set `self.Death Niagara System` DeathNiagaraSystem)
  (`|ExecutionSequence`
    (:`then_0`
      (set `SkeletalMeshComponent.bPauseAnims` true (`self.Mesh`))
      (`PrimitiveComponent.SetCollisionEnabled` (`self.CapsuleComponent`) "NoCollision"))
    (:`then_1`
      (bind _object (`|LoadAsset` (`self.Death Niagara System`))
        (:`Completed`
          (bind `_as나이아가라_시스템` (cast `NiagaraSystem` _object))
          (bind _returnvalue (`NiagaraFunctionLibrary.SpawnSystemAttached` `_as나이아가라_시스템` (`self.Mesh`) "None" (0.0 0.0 0.0) (struct) "KeepRelativeOffset" true))
          (set `self.DeathNiagaraParticleSystem` _returnvalue)
          (bind _returnvalue_2 (`PrimitiveComponent.CreateDynamicMaterialInstance` _mesh 0 (`PrimitiveComponent.GetMaterial` _mesh 0) "None"))
          (bind _returnvalue_3 (`MaterialInstanceDynamic.K2_GetVectorParameterValue` _returnvalue_2 "DissolveEdgeColor"))
          (`NiagaraComponent.SetNiagaraVariableLinearColor` (`self.DeathNiagaraParticleSystem`) "DissolveParticleColor" _returnvalue_3))))
    (:`then_2`
      (`TimelineComponent.SetPlayRate` (`self.DissolveActorTimeline`) (/ 1.0 (`self.DissolveActorTime`)))
      (bind (_direction _dissolveamount) (`Timeline|DissolveActorTimeline` :!via `PlayFromStart`)
        (:`Update`
          (`MeshComponent.SetScalarParameterValueOnMaterials` (`self.Mesh`) "DissolveAmount" _dissolveamount))
        (:`Finished`
          (`self.K2_DestroyActor`))))
    (:`then_3`
      (`TimelineComponent.SetPlayRate` (`self.DissolveWeaponTimeline`) (/ 1.0 (`self.DissolveWeaponTime`)))
      (bind (_direction_2 _dissolveamount_2) (`Timeline|DissolveWeaponTimeline` :!via `PlayFromStart`)
        (:`Update`
          (`/Engine/EditorBlueprintResources/StandardMacros.IsValid` _weaponmesh
            (:`Is Valid`
              (`MeshComponent.SetScalarParameterValueOnMaterials` _weaponmesh "DissolveAmount" _dissolveamount_2))))
        (:`Finished`
          (`self.K2_DestroyActor` (`PawnCombatComponent.GetCurrentEquippedWeapon` (`self.EnemyCombatComponent`))))))))

(fn `UserConstructionScript`)