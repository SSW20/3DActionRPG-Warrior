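; Shared projectile Blueprint that handles the sound and Niagara effects for a projectile's spawn, flight and impact.
; BeginPlay plays a spawn sound at the actor's location and attaches a looping-agnostic fly sound and effect oriented along its forward vector.
; ProjectileHit receives an impact point, stores it, and plays the optional hit sound and effect there.
; Movement, collision detection and damage are absent from these graphs.
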(event `self.ReceiveBeginPlay`
  (`|ExecutionSequence`
    (:`then_0`
      (`GameplayStatics.PlaySoundAtLocation` (`self.SpawnSound`) (`self.K2_GetActorLocation`) (struct) 1.0 1.0 0.0 null null null null))
    (:`then_1`
      (`GameplayStatics.SpawnSoundAttached` (`self.FlySound`) (`self.RootComponent`) "None" (0.0 0.0 0.0) (struct) "KeepRelativeOffset" true 1.0 1.0 0.0 null null))
    (:`then_2`
      (`NiagaraFunctionLibrary.SpawnSystemAttached` (`self.FlyFX`) null "None" (`self.K2_GetActorLocation`) (`KismetMathLibrary.MakeRotFromX` (`self.GetActorForwardVector`)) "KeepRelativeOffset"))))

(event `self.ProjectileHit`
  (params (ImpactPoint :type "Vector Structure (by ref)"))
  (set `self.Impact Point` ImpactPoint)
  (`|ExecutionSequence`
    (:`then_0`
      (bind _hitsound (`self.HitSound`)
        (:`then`
          (`GameplayStatics.PlaySoundAtLocation` _hitsound (`self.Impact Point`) (struct) 1.0 1.0 0.0 null null null null))
        (:`else`)))
    (:`then_1`
      (bind _hiteffect (`self.HitEffect`)
        (:`then`
          (`NiagaraFunctionLibrary.SpawnSystemAtLocation` _hiteffect (`self.Impact Point`)))
        (:`else`)))))

(fn `UserConstructionScript`)